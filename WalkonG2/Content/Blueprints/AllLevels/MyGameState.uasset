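; MyGameState is a game state Blueprint that holds the team material taken from the first player controller's settings.
; On BeginPlay, and again whenever its Update event fires, it casts player controller 0 to GameplayPC and copies PlayerSettings.TeamMaterial into MaterialTeam.
; An authority check casting to GameplayGM and some debug prints remain as disconnected, unused nodes.
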(event Custom|Update
  (bind _asgameplay_pc (Utilities|Casting|CastToGameplayPC (Game|GetPlayerController 0)))
  (Variables|Default|SetMaterialTeam (.TeamMaterial (Utilities|Struct|BreakPlayerInfo (Variables|/Game/Blueprints/Gameplay/GameplayPC.GameplayPC_C|GetPlayerSettings _asgameplay_pc)))))

(event EventBeginPlay
  (bind _asgameplay_pc (Utilities|Casting|CastToGameplayPC (Game|GetPlayerController 0)))
  (Variables|Default|SetMaterialTeam (.TeamMaterial (Utilities|Struct|BreakPlayerInfo (Variables|/Game/Blueprints/Gameplay/GameplayPC.GameplayPC_C|GetPlayerSettings _asgameplay_pc)))))

(fn ConstructionScript
  (|CallParentFunction))