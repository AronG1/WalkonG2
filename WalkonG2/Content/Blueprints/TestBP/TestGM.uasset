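; Test multiplayer game mode that manages player spawning, character swapping and kill/death scoreboard data.
; On server login it registers the controller, caches PlayerStarts, sets up its widget, possesses it with a ghost at a fixed location and zeroes its stats.
; SwapCharacter, when ChangeStatus is false, replaces the pawn with the given class at a random PlayerStart.
; FillAllPlayersInfo rebuilds the scoreboard array from each TestPC's PlayerKD.
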(event Custom|SpawnGhost
  (params (PlayerController :type Player%20Controller%20Object%20Reference))
  (bind _returnvalue (Pawn|GetControlledPawn PlayerController))
  ;[1 1 1] Spawn ghost
  (Utilities|IsValid _returnvalue
    (:Is%20Valid
      (Actor|DestroyActor _returnvalue))
    (:Is%20Not%20Valid
      _))
  (bind _returnvalue_2 (Game|SpawnActorfromClass "/Game/Blueprints/TestBP/GhostCharacter.GhostCharacter_C" (Math|Transform|MakeTransform "940.000000,600.000000,315.000000") "Undefined" 0 0))
  (Pawn|Possess PlayerController _returnvalue_2)
  ;[0.25 0.007955 0] Fail to scoreboard
  (CallFunction|InitializePlayerInfo))

(event Custom|InitializePlayerInfo
  ;[0.25 0.007955 0] Fail to scoreboard
  (bind _astest_pc (Utilities|Casting|CastToTestPC (stale Custom|SpawnGhost PlayerController))
    (:then
      (bind _structout (Utilities|Struct|SetmembersinPlayerKD (Variables|/Game/Blueprints/TestBP/TestPC.TestPC_C|GetPlayerKD _astest_pc)))
      (Variables|/Game/Blueprints/TestBP/TestPC.TestPC_C|SetPlayerKD _astest_pc _structout))
    (:CastFailed
      (Development|PrintString "cast failed"))))

(event Custom|SwapCharacter
  (params (PlayerController :type Player%20Controller%20Object%20Reference) (CharacterClass :type Character%20Class%20Reference) (ChangeStatus :type Boolean))
  (bind _returnvalue (Pawn|GetControlledPawn PlayerController))
  (bind _playerstarts (Variables|Default|GetPlayerStarts))
  ;[1 1 1] Swap character
  (if (not ChangeStatus)
    (Utilities|IsValid _returnvalue
      (:Is%20Valid
        (Actor|DestroyActor _returnvalue))
      (:Is%20Not%20Valid
        _))
    (bind _returnvalue_2 (Game|SpawnActorfromClass CharacterClass (Math|Transform|MakeTransform (Transformation|GetActorLocation (Utilities|Array|Get(acopy) _playerstarts (Math|Random|RandomIntegerinRange 0 (- (Utilities|Array|Length _playerstarts) 1))))) "Undefined" 0 0))
    (Pawn|Possess PlayerController _returnvalue_2)
    (bind _astest_pc (Utilities|Casting|CastToTestPC PlayerController))
    (Networking|SwitchHasAuthority
      (:Authority
        (Default|InputModeGameOnlyandAddStartMessage _astest_pc)))))

(event Custom|FillAllPlayersInfo
  ;[0.25 0.007955 0] Fail to scoreboard
  (Utilities|Array|Clear (Variables|Default|GetAllPlayersInfo))
  (for _array_element (Variables|Default|GetAllPlayerControllers)
    (bind _astest_pc (Utilities|Casting|CastToTestPC _array_element))
    (Utilities|Array|Add (Variables|Default|GetAllPlayersInfo) (Variables|/Game/Blueprints/TestBP/TestPC.TestPC_C|GetPlayerKD _astest_pc))))

(event EventPostLogin
  (params (NewPlayer :type Player%20Controller%20Object%20Reference))
  ;[1 1 1] On log in
  (Networking|SwitchHasAuthority
    (:Authority
      (Utilities|Array|Add (Variables|Default|GetAllPlayerControllers) NewPlayer)
      (bind _outactors (Actor|GetAllActorsOfClass "/Script/Engine.PlayerStart"))
      (Variables|Default|SetPlayerStarts _outactors)
      (bind _astest_pc (Utilities|Casting|CastToTestPC NewPlayer))
      (bind _output_get (Variables|Default|SetPlayerController _astest_pc))
      (Default|SetupWidget _output_get)
      (CallFunction|SpawnGhost NewPlayer))))

(fn ConstructionScript)