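; Poison arrow projectile for Erika that deals hit damage, then repeated poison damage.
; On its first hit, the server capsule-traces forward for the bone, applies headshot or random body damage and attaches the arrow mesh there.
; A looping timer reapplies poison damage up to a tick limit.
; Bone hits add money to the shooter's GameplayPC, or subtract it for teammates, who still take damage.
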(event OnComponentHit(SphereCollision)
  (params (HitComponent :type Primitive%20Component%20Object%20Reference) (OtherActor :type Actor%20Object%20Reference) (OtherComp :type Primitive%20Component%20Object%20Reference) (NormalImpulse :type Vector :default "0, 0, 0") (Hit :type Hit%20Result%20Structure%20%28by%20ref%29))
  (Networking|SwitchHasAuthority
    (:Authority
      (Utilities|FlowControl|DoOnce false
        (:Completed
          (CallFunction|CalculateTrace)
          (CallFunction|ApplyDamage)
          (CallFunction|AttachArrowAll)
          (CallFunction|SetTimer)
          (if (Variables|Default|GetIsActor)
            (CallFunction|CheckTeammate)
            (if (Variables|Default|GetIsTeammate)
              (CallFunction|SubtractMoney (Variables|Default|GetMoneyToAdd))
              (else
                (CallFunction|AddMoney (Variables|Default|GetMoneyToAdd))))))))))

(event Custom|AttachArrowAll
  (CallFunction|AttachArrow))

(event Custom|SetTimer
  (bind _returnvalue (Utilities|Time|SetTimerbyFunctionName 0 "ApplyPoisonDamage" 1.0 true)))

(event Custom|SubtractMoney
  (params (Money :type Integer))
  ;[1 1 1] Server tells client to subtract money
  (bind _asgameplay_pc (Utilities|Casting|CastToGameplayPC (Game|GetInstigatorController))
    (:then
      (Default|SubtractMoney _asgameplay_pc Money))
    (:CastFailed
      (Development|PrintString "CAST FAILED:: no gameplayPC from arrrow" true true "(R=1.000000,G=0.000000,B=0.047119,A=1.000000)" 2e+01))))

(event Custom|StopTimer
  (Utilities|Time|ClearandInvalidateTimerbyHandle (stale Custom|SetTimer _returnvalue)))

(event Custom|AddMoney
  (params (Money :type Integer))
  ;[1 1 1] Server tells client to add money
  (bind _asgameplay_pc (Utilities|Casting|CastToGameplayPC (Game|GetInstigatorController))
    (:then
      (Default|AddMoney _asgameplay_pc Money))
    (:CastFailed
      (Development|PrintString "CAST FAILED:: no gameplayPC from arrrow" true true "(R=1.000000,G=0.000000,B=0.047119,A=1.000000)" 2e+01))))

(event EventBeginPlay)

(event Collision|EventActorBeginOverlap
  (params (OtherActor :type Actor%20Object%20Reference)))

(event EventTick
  (params (DeltaSeconds :type Float%20%28single-precision%29)))

(fn ConstructionScript)

(fn CalculateTrace
  (bind _spherecollision (Variables|Default|GetSphereCollision))
  (bind _returnvalue (Transformation|GetWorldLocation _spherecollision))
  (Networking|SwitchHasAuthority
    (:Authority
      (bind (_outhit _returnvalue_2) (Collision|CapsuleTraceByChannel _returnvalue (+ _returnvalue (* (Math|Vector|GetForwardVector (Transformation|GetWorldRotation _spherecollision)) 1e+02)) 0.0 0.0 "TraceTypeQuery1" false 0 "Persistent"))
      (bind _output_get (Variables|Default|SetHitResults _outhit))
      (if _returnvalue_2
        (if (Utilities|Name|NotEqual(Name) (.HitBoneName (Collision|BreakHitResult _output_get)) "")
          (Variables|Default|SetIsActor true)
          (Components|Movement|StopMovementImmediately (Variables|Default|GetProjectileMovement))
          (else
            (Variables|Default|SetIsActor false)))
        (Transformation|SetActorLocation (.ImpactPoint (Collision|BreakHitResult _output_get)) false false)))))

(fn ApplyDamage
  (bind _hitresults (Variables|Default|GetHitResults))
  (bind (_bblockinghit _binitialoverlap _time _location _impactpoint _normal _impactnormal _physmat _hitactor _hitcomponent _hitbonename) (Collision|BreakHitResult _hitresults))
  (if (Utilities|Name|Equal(Name) _hitbonename "Head")
    (Variables|Default|SetDamage 1e+02)
    (Variables|Default|SetMoneyToAdd (Variables|Default|GetHeadshotMoney))
    (else
      (Variables|Default|SetDamage (Math|Random|RandomFloatinRange 45.0 55.0))
      (Variables|Default|SetMoneyToAdd (Variables|Default|GetHitMoney))))
  (Game|Damage|ApplyDamage _hitactor (Variables|Default|GetDamage) (Game|GetInstigatorController) self (Variables|Default|GetDamageType)))

(fn AttachArrow
  (bind _hitresults (Variables|Default|GetHitResults))
  (bind (_bblockinghit _binitialoverlap _time _location _impactpoint _normal _impactnormal _physmat _hitactor _hitcomponent _hitbonename) (Collision|BreakHitResult _hitresults))
  (Transformation|AttachComponentToComponent (Variables|Default|GetArrowMesh) _hitcomponent _hitbonename "KeepWorld" "KeepWorld" "KeepWorld" true))

(fn ApplyPoisonDamage
  (Variables|Default|SetDamage (Variables|Default|GetPoisonDamage))
  (Game|Damage|ApplyDamage (.HitActor (Collision|BreakHitResult (Variables|Default|GetHitResults))) (Variables|Default|GetDamage) (Game|GetInstigatorController) self (Variables|Default|GetDamageType))
  (Variables|Default|SetNumOfFireDamage (+ (Variables|Default|GetNumOfFireDamage) 1))
  (if (>= (Variables|Default|GetNumOfFireDamage) (Variables|Default|GetMaxNumOfFireDamage))
    (CallFunction|StopTimer)))

(fn CheckTeammate
  (Networking|SwitchHasAuthority
    (:Authority
      (bind _asgameplay_pc (Utilities|Casting|CastToGameplayPC (Game|GetInstigatorController))
        (:then
          (bind _asgameplay_pc_2 (Utilities|Casting|CastToGameplayPC (Game|GetInstigatorController (.HitActor (Collision|BreakHitResult (Variables|Default|GetHitResults)))))
            (:then
              (if (== (.TeamID (Utilities|Struct|BreakPlayerInfo (Variables|/Game/Blueprints/Gameplay/GameplayPC.GameplayPC_C|GetPlayerSettings _asgameplay_pc))) (.TeamID (Utilities|Struct|BreakPlayerInfo (Variables|/Game/Blueprints/Gameplay/GameplayPC.GameplayPC_C|GetPlayerSettings _asgameplay_pc_2))))
                (Variables|Default|SetIsTeammate true)
                (else
                  (Variables|Default|SetIsTeammate false))))
            (:CastFailed
              (Development|PrintString "CAST FAILED:: no gmPC here  2" true true "(R=0.000000,G=0.660000,B=1.000000,A=1.000000)" 2e+01))))
        (:CastFailed
          (Development|PrintString "CAST FAILED:: no gmPC here" true true "(R=0.000000,G=0.660000,B=1.000000,A=1.000000)" 2e+01))))))