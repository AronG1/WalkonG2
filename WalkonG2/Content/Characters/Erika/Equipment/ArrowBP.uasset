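; Arrow projectile that damages what it hits and sticks into it, with hit logic starting on the server.
; The first sphere collision hit runs a forward capsule trace that moves the arrow to the impact point, stopping movement when a bone is hit.
; Head bone hits deal fixed high damage, others a random lower amount, then the mesh attaches to the hit component at that bone.
; Debug trace drawing and an instigator printout remain active.
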(event OnComponentHit(SphereCollision)
  (params (HitComponent :type Primitive%20Component%20Object%20Reference) (OtherActor :type Actor%20Object%20Reference) (OtherComp :type Primitive%20Component%20Object%20Reference) (NormalImpulse :type Vector :default "0, 0, 0") (Hit :type Hit%20Result%20Structure%20%28by%20ref%29))
  (Networking|SwitchHasAuthority
    (:Authority
      (Utilities|FlowControl|DoOnce false
        (:Completed
          (CallFunction|CalculateTrace)
          (CallFunction|ApplyDamage)
          (CallFunction|AttachArrowAll))))))

(event Custom|AttachArrowAll
  (CallFunction|AttachArrow))

(event EventBeginPlay)

(event Collision|EventActorBeginOverlap
  (params (OtherActor :type Actor%20Object%20Reference)))

(event EventTick
  (params (DeltaSeconds :type Float%20%28single-precision%29)))

(fn ConstructionScript)

(fn CalculateTrace
  (bind _spherecollision (Variables|Default|GetSphereCollision))
  (bind _returnvalue (Transformation|GetWorldLocation _spherecollision))
  (Networking|SwitchHasAuthority
    (:Authority
      (bind (_outhit _returnvalue_2) (Collision|CapsuleTraceByChannel _returnvalue (+ _returnvalue (* (Math|Vector|GetForwardVector (Transformation|GetWorldRotation _spherecollision)) 1e+02)) 0.0 0.0 "TraceTypeQuery1" false 0 "Persistent"))
      (bind _output_get (Variables|Default|SetHitResults _outhit))
      (if _returnvalue_2
        (if (Utilities|Name|NotEqual(Name) (.HitBoneName (Collision|BreakHitResult _output_get)) "")
          (Components|Movement|StopMovementImmediately (Variables|Default|GetProjectileMovement)))
        (Transformation|SetActorLocation (.ImpactPoint (Collision|BreakHitResult _output_get)) false false)))))

(fn ApplyDamage
  (bind _returnvalue (Game|GetInstigatorController))
  (bind _hitresults (Variables|Default|GetHitResults))
  (bind (_bblockinghit _binitialoverlap _time _location _impactpoint _normal _impactnormal _physmat _hitactor _hitcomponent _hitbonename) (Collision|BreakHitResult _hitresults))
  (Networking|SwitchHasAuthority
    (:Authority
      (if (Utilities|Name|Equal(Name) _hitbonename "Head")
        (Variables|Default|SetDamage 1e+02)
        (else
          (Variables|Default|SetDamage (Math|Random|RandomFloatinRange 35.0 4e+01))))
      (Game|Damage|ApplyDamage _hitactor (Variables|Default|GetDamage) _returnvalue self (Variables|Default|GetDamageType))
      (Development|PrintString (Utilities|GetDisplayName _returnvalue) true true "(R=1.000000,G=0.926994,B=0.000000,A=1.000000)" 5e+01))))

(fn AttachArrow
  (bind _hitresults (Variables|Default|GetHitResults))
  (bind (_bblockinghit _binitialoverlap _time _location _impactpoint _normal _impactnormal _physmat _hitactor _hitcomponent _hitbonename) (Collision|BreakHitResult _hitresults))
  (Transformation|AttachComponentToComponent (Variables|Default|GetArrowMesh) _hitcomponent _hitbonename "KeepWorld" "KeepWorld" "KeepWorld" true))