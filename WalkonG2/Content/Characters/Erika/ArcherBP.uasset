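; Networked playable archer character (Erika) with aimed bow shots, sprint, kick, team material and purchasable poison and fire arrow upgrades.
; Aiming requires arrows and energy, and its RepNotify toggles shoot camera and crosshair.
; Leaving aim fires from that camera, spending both resources; timed energy regeneration pauses while sprinting.
; Authority-side damage picks arrow or sword montages, while GameplayPC handles money, chat and the respawn widget on death or class change.
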(event Custom|ArrowVisibiilityOff
  ;[1 1 1] Arrow visibility
  (Rendering|SetVisibility (Variables|Default|GetTheArrow) false false))

(event Custom|SetAimCamera
  ;[1 1 1] Set aim camera on to everyone
  (Components|Activation|SetActive (Variables|Default|GetCamera) false false)
  (Components|Activation|SetActive (Variables|Default|GetShootCam) true false))

(event Custom|ArrowImpact
  ;[1 1 1] Play arrow impact anim
  (Animation|PlayAnimMontage (Variables|AnimMontages|GetArrowImpactAnimMontage) 1.0 "None"))

(event Custom|SwordImpact
  ;[1 1 1] Play sword impact anim
  (Animation|PlayAnimMontage (Variables|AnimMontages|GetSwordAnimMontage) 1.0 "None"))

(event Custom|BodyRotationServer
  ;[1 1 1] Call calculateBodyRot function
  (CallFunction|CalculateBodyRotation))

(event Custom|ArrowDeath
  ;[1 1 1] Play arrow death anim
  (Variables|AnimMontages|SetDeathAnimMontage (Variables|AnimMontages|GetArrowDeathAnimMontage))
  (CallFunction|Death))

(event Custom|SwordDeath
  ;[1 1 1] Play sword death anim
  (Variables|AnimMontages|SetDeathAnimMontage (Variables|AnimMontages|GetSwordDeathAnimMontage))
  (CallFunction|Death))

(event Custom|ShootArrow
  ;[1 1 1] Shooting arrow
  (CallFunction|SpawnArrow))

(event Custom|ClearAim
  ;[1 1 1] set isAim var to off
  (Variables|CharacterStatus|SetIsAim false)
  (CallFunction|CalculateArrowTransform)
  (CallFunction|ShootArrow)
  (CallFunction|ArrowVisibiilityOff)
  (CallFunction|EnergySpend)
  (CallFunction|ArrowSpend))

(event Custom|AddArrows
  ;[1 1 1] Adds arrows from cubeArrows
  (Networking|SwitchHasAuthority
    (:Authority
      (Variables|Attributes|SetNumOfArrows (Variables|GameplaySettings|GetMaxNumOfArrows)))))

(event Custom|ClearAimCamera
  ;[1 1 1] Set aim camera off to everyone
  (Components|Activation|SetActive (Variables|Default|GetCamera) true false)
  (Components|Activation|SetActive (Variables|Default|GetShootCam) false false))

(event Custom|SetTeamMaterial
  (params (Material :type Material%20Interface%20Object%20Reference))
  ;[1 1 1] Server sets material and says to everyone to do it
  (Variables|Material|SetTeamMaterial Material)
  (Rendering|Material|SetMaterial (Variables|Character|GetMesh) 0 (Variables|Material|GetTeamMaterial))
  (CallFunction|SetMaterialAll))

(event Custom|StartSprint
  ;[1 1 1] Sprint
  (CallFunction|Sprint)
  (CallFunction|StopRestoreEnergy))

(event Custom|EnergyRestore
  ;[1 1 1] Energy restore
  (bind _returnvalue (Utilities|Time|SetTimerbyFunctionName 0 "RestoreEnergy" 0.5 true)))

(event Custom|StopRestoreEnergy
  ;[1 1 1] Energy restore
  (Utilities|Time|ClearandInvalidateTimerbyHandle (stale Custom|EnergyRestore _returnvalue)))

(event Custom|StartSprintAll
  ;[1 1 1] Sprint
  (CallFunction|SprintAll))

(event Custom|StopSprint
  ;[1 1 1] Sprint
  (CallFunction|Walk)
  (CallFunction|EnergyRestore))

(event Custom|StopSprintAll
  ;[1 1 1] Sprint
  (CallFunction|WalkAll))

(event Custom|FirstAbilityServer
  ;[1 1 1] Arrow ability
  (bind _hasmoney (CallFunction|HasEnoughMoney))
  (if _hasmoney
    (bind _money (CallFunction|SetArrowType))
    (CallFunction|SubtractMoney _money)))

(event Custom|CreateAimWidget
  ;[1 1 1] Add Aim Widget
  (CallFunction|AddCrosshair))

(event Custom|KickServer
  ;[1 1 1] Kick
  (Animation|PlayAnimMontage (Variables|AnimMontages|GetKickAnimMontage) 1.0 "None")
  (CallFunction|KickAll))

(event Custom|SubtractMoney
  (params (Money :type Integer))
  ;[1 1 1] Arrow ability
  (bind _asgameplay_pc (Utilities|Casting|CastToGameplayPC (Game|GetInstigatorController)))
  (Default|SubtractMoney _asgameplay_pc Money))

(event Custom|KickAll
  ;[1 1 1] Kick
  (Animation|PlayAnimMontage (Variables|AnimMontages|GetKickAnimMontage) 1.0 "None"))

(event Custom|RemoveAimWidget
  ;[1 1 1] Remove aim Widget
  (CallFunction|RemoveCrosshair))

(event Custom|SetAim
  ;[1 1 1] Server check for arrows and energy, set isAim to on
  (bind _hasarrows (CallFunction|HasArrows))
  (if _hasarrows
    (bind _hasenergy (CallFunction|HasEnergy))
    (if _hasenergy
      (Variables|CharacterStatus|SetIsAim true))))

(event Custom|ChangeClass
  ;[1 1 1] Change class
  (Variables|CharacterStatus|SetIsAlive false)
  (CallFunction|SwordDeath)
  (CallFunction|Respawn))

(event Custom|Respawn
  ;[1 1 1] Respawn
  (bind _asgameplay_pc (Utilities|Casting|CastToGameplayPC (Game|GetPlayerController 0)))
  (Default|SetupWidget _asgameplay_pc))

(event Custom|CallMaterialFunction
  ;[1 1 1] Call material function from owning client
  (CallFunction|TeamColor))

(event Custom|SetMaterialAll
  ;[1 1 1] Everyone sets material
  (Rendering|Material|SetMaterial (Variables|Character|GetMesh) 0 (Variables|Material|GetTeamMaterial)))

(event Custom|AddHUD
  ;[1 1 1] Adding HUD to viewport
  (bind _returnvalue (UserInterface|CreateWidget (Variables|Widgets|GetArcherHUDClass)))
  (bind _output_get (Variables|Widgets|SetArcherHUD _returnvalue))
  (UserInterface|Viewport|AddtoViewport _output_get 0))

(event Custom|ArrowVisibilityOn
  ;[1 1 1] Arrow visibility
  (Rendering|SetVisibility (Variables|Default|GetTheArrow) true false))

(event EventPossessed
  (params (NewController :type Controller%20Object%20Reference))
  ;[1 1 1] Initialization
  (Networking|SwitchHasAuthority
    (:Authority
      (CallFunction|Initialization)
      ;[1 1 1] Add HUD
      (CallFunction|AddHUD))))

(event Game|Damage|EventAnyDamage
  (params (Damage :type Float%20%28single-precision%29) (DamageType :type Damage%20Type%20Object%20Reference) (InstigatedBy :type Controller%20Object%20Reference) (DamageCauser :type Actor%20Object%20Reference))
  ;[1 1 1] Recive damage
  (CallFunction|HandleDamage Damage DamageType InstigatedBy DamageCauser))

(event Input|ActionEvents|InputActionWriteKey
  (params (Key :type Key%20Structure :default "AnyKey"))
  ;[1 1 1] Writing in chat
  (:Pressed
    (bind _asgameplay_pc (Utilities|Casting|CastToGameplayPC (Game|GetPlayerController 0)))
    (Default|SwitchtoWrite _asgameplay_pc)))

(event Input|ActionEvents|InputActionAttack
  (params (Key :type Key%20Structure :default "AnyKey"))
  ;[1 1 1] Asking server to aim/clear aim
  (:Pressed
    (if (Variables|CharacterStatus|GetIsAlive)
      (if (Variables|PlayerSettings|GetIsAimHold)
        (if (not (Variables|CharacterStatus|GetIsAim))
          (bind _hasarrows (CallFunction|HasArrows :!label _label))
          (if _hasarrows
            (bind _hasenergy (CallFunction|HasEnergy))
            (if _hasenergy
              (CallFunction|SetAim))))
        (elif (Variables|CharacterStatus|GetIsAim)
          (CallFunction|ClearAim)
          (else
            (goto _label))))))
  (:Released
    (if (Variables|PlayerSettings|GetIsAimHold)
      (if (Variables|CharacterStatus|GetIsAlive)
        (CallFunction|ClearAim)))))

(event Input|ActionEvents|InputActionSprint
  (params (Key :type Key%20Structure :default "AnyKey"))
  ;[1 1 1] Sprint
  (:Pressed
    (if (not (Variables|CharacterStatus|GetIsAim))
      (CallFunction|StartSprint)))
  (:Released
    (CallFunction|StopSprint)))

(event Input|ActionEvents|InputActionFirstAbility
  (params (Key :type Key%20Structure :default "AnyKey"))
  ;[1 1 1] Arrow ability
  (:Pressed
    (bind _hasmoney (CallFunction|HasEnoughMoney))
    (if _hasmoney
      (CallFunction|FirstAbilityServer))))

(event Input|ActionEvents|InputActionKick
  (params (Key :type Key%20Structure :default "AnyKey"))
  ;[1 1 1] Kick
  (:Pressed
    (CallFunction|KickServer)))

(event Input|ActionEvents|InputActionChangePlayer
  (params (Key :type Key%20Structure :default "AnyKey"))
  ;[1 1 1] Change class
  (:Pressed
    (CallFunction|ChangeClass)))

(event Input|AxisEvents|InputAxisMoveForward
  (params (AxisValue :type Float%20%28single-precision%29))
  ;[1 1 1] Movement
  (if (Variables|CharacterStatus|GetIsAlive)
    (Pawn|Input|AddMovementInput (Math|Vector|GetForwardVector (Math|Rotator|MakeRotator 0.0 0.0 (.Yaw (Math|Rotator|BreakRotator (Pawn|GetControlRotation :!class /Script/Engine.Pawn))))) AxisValue false)))

(event Input|AxisEvents|InputAxisTurn
  (params (AxisValue :type Float%20%28single-precision%29))
  ;[1 1 1] Turn
  (if (Variables|CharacterStatus|GetIsAlive)
    (Pawn|Input|AddControllerYawInput AxisValue)))

(event Input|AxisEvents|InputAxisMoveRight
  (params (AxisValue :type Float%20%28single-precision%29))
  ;[1 1 1] Movement
  (if (Variables|CharacterStatus|GetIsAlive)
    (Pawn|Input|AddMovementInput (Math|Vector|GetRightVector (Math|Rotator|MakeRotator 0.0 0.0 (.Yaw (Math|Rotator|BreakRotator (Pawn|GetControlRotation :!class /Script/Engine.Pawn))))) AxisValue false)))

(event Input|AxisEvents|InputAxisLookUp
  (params (AxisValue :type Float%20%28single-precision%29))
  ;[1 1 1] Look up / inverse look
  (if (Variables|CharacterStatus|GetIsAlive)
    (if (Variables|PlayerSettings|GetIsInverseLook?)
      (Pawn|Input|AddControllerPitchInput AxisValue)
      (else
        (Pawn|Input|AddControllerPitchInput (* AxisValue -1.0))))))

(fn ConstructionScript)

(fn Initialization
  (Networking|SwitchHasAuthority
    (:Authority
      (Variables|CharacterStatus|SetIsAlive true)
      (Variables|Attributes|SetHealth (Variables|GameplaySettings|GetMaxHealth))
      (Variables|Attributes|SetEnergy (Variables|GameplaySettings|GetMaxEnergy))
      (Variables|Attributes|SetNumOfArrows (Variables|GameplaySettings|GetMaxNumOfArrows))
      (Variables|Classes|SetArrowClass (Variables|Classes|GetNormalArrowClass))
      (Variables|CharacterStatus|SetIsAim false)
      (CallFunction|EnergyRestore)
      (CallFunction|CallMaterialFunction))))

(fn Sprint
  (Networking|SwitchHasAuthority
    (:Authority
      (if (not (Variables|CharacterStatus|GetIsAim))
        (Variables|/Script/Engine.CharacterMovementComponent|SetMaxWalkSpeed (Variables|Character|GetCharacterMovement) (Variables|GameplaySettings|GetMaxSprintSpeed))
        (CallFunction|StartSprintAll)))))

(fn SprintAll
  (Variables|/Script/Engine.CharacterMovementComponent|SetMaxWalkSpeed (Variables|Character|GetCharacterMovement) (Variables|GameplaySettings|GetMaxSprintSpeed)))

(fn Walk
  (Networking|SwitchHasAuthority
    (:Authority
      (Variables|/Script/Engine.CharacterMovementComponent|SetMaxWalkSpeed (Variables|Character|GetCharacterMovement) (Variables|GameplaySettings|GetMaxWalkSpeed))
      (CallFunction|StopSprintAll))))

(fn WalkAll
  (Variables|/Script/Engine.CharacterMovementComponent|SetMaxWalkSpeed (Variables|Character|GetCharacterMovement) (Variables|GameplaySettings|GetMaxWalkSpeed)))

(fn HasArrows
  (return (> (Variables|Attributes|GetNumOfArrows) 0)))

(fn HasEnergy
  (return (>= (Variables|Attributes|GetEnergy) (Variables|GameplaySettings|GetEnergySpendToShootArrow))))

(fn OnRepIsAim
  (bind _shootcam (Variables|Default|GetShootCam))
  (bind _camera (Variables|Default|GetCamera))
  (Networking|SwitchHasAuthority
    (:Authority
      (if (Variables|CharacterStatus|GetIsAim)
        (Components|Activation|SetActive _camera false false)
        (Components|Activation|SetActive _shootcam true false)
        (CallFunction|SetAimCamera)
        (CallFunction|CreateAimWidget)
        (else
          (Components|Activation|SetActive _camera true false)
          (Components|Activation|SetActive _shootcam false false)
          (CallFunction|ClearAimCamera)
          (CallFunction|RemoveAimWidget))))))

(fn AddCrosshair
  (bind _returnvalue (UserInterface|CreateWidget (Variables|Widgets|GetCrosshairWidgetClass)))
  (bind _output_get (Variables|Widgets|SetCrosshairWidget _returnvalue))
  (UserInterface|Viewport|AddtoViewport _output_get 0))

(fn RemoveCrosshair
  (Widget|RemovefromParent (Variables|Widgets|GetCrosshairWidget)))

(fn CalculateBodyRotation
  (Networking|SwitchHasAuthority
    (:Authority
      (Variables|CharacterStatus|SetBodyRotation (Math|Rotator|MakeRotator (* (Math|Float|ClampAngle (.pitch (Pawn|GetControlRotation :!class /Script/Engine.Pawn)) -45.0 45.0) -1.0) 0.0 0.0)))))

(fn HandleDamage
  (params (Damage :type Float%20%28single-precision%29) (DamageType :type Damage%20Type%20Object%20Reference) (Instigated :type Controller%20Object%20Reference) (DamageCauser :type Actor%20Object%20Reference))
  (Networking|SwitchHasAuthority
    (:Authority
      (Variables|Damage|SetDamageType DamageType)
      (Variables|Damage|SetInstigated Instigated)
      (Variables|Damage|SetDamageCauser DamageCauser)
      (if (Variables|CharacterStatus|GetIsAlive)
        (Variables|Attributes|SetHealth (- (Variables|Attributes|GetHealth) Damage))
        (if (> (Variables|Attributes|GetHealth) 0.0)
          (if (== (Utilities|GetClass (Variables|Damage|GetDamageType)) "/Game/Blueprints/AllLevels/ArrowDamage.ArrowDamage_C")
            (CallFunction|ArrowImpact)
            (Utilities|Array|Add (Variables|Default|GetArrows) (Variables|Damage|GetDamageCauser))
            (else
              (CallFunction|SwordImpact)))
          (else
            (Variables|CharacterStatus|SetIsAlive false)
            (if (== (Utilities|GetClass (Variables|Damage|GetDamageType)) "/Game/Blueprints/AllLevels/ArrowDamage.ArrowDamage_C")
              (CallFunction|ArrowDeath)
              (else
                (CallFunction|SwordDeath)))
            (CallFunction|Respawn)))))))

(fn SpawnArrow
  (Game|SpawnActorfromClass (Variables|Classes|GetArrowClass) (Variables|Variables|GetArrowTransform) "Undefined" self (Game|GetInstigator)))

(fn CalculateArrowTransform
  (bind _shootcam (Variables|Default|GetShootCam))
  (bind _returnvalue (Transformation|GetWorldTransform _shootcam))
  (Networking|SwitchHasAuthority
    (:Authority
      (Variables|Variables|SetArrowTransform (Math|Transform|MakeTransform (+ (.location _returnvalue) (* (Math|Vector|GetForwardVector _shootcam) 1e+02)) (.rotation _returnvalue) (.scale _returnvalue))))))

(fn Death
  (Animation|PlayAnimMontage (Variables|AnimMontages|GetDeathAnimMontage) 1.0 "None"))

(fn RestoreEnergy
  (Variables|Attributes|SetEnergy (Math|Float|Clamp(Float) (+ (Variables|Attributes|GetEnergy) (Variables|GameplaySettings|GetEnergyRestoreAdd)) 0.0 1e+02)))

(fn EnergySpend
  (Networking|SwitchHasAuthority
    (:Authority
      (Variables|Attributes|SetEnergy (- (Variables|Attributes|GetEnergy) (Variables|GameplaySettings|GetEnergySpendToShootArrow))))))

(fn ArrowSpend
  (Networking|SwitchHasAuthority
    (:Authority
      (Variables|Attributes|SetNumOfArrows (- (Variables|Attributes|GetNumOfArrows) 1)))))

(fn TeamColor
  (bind _asgameplay_pc (Utilities|Casting|CastToGameplayPC (Game|GetPlayerController 0)))
  (CallFunction|SetTeamMaterial (.TeamMaterial (Utilities|Struct|BreakPlayerInfo (Variables|/Game/Blueprints/Gameplay/GameplayPC.GameplayPC_C|GetPlayerSettings _asgameplay_pc)))))

(fn SetArrowType
  (Networking|SwitchHasAuthority
    (:Authority
      (switch int (Variables|Money|GetSwitchAbility)
        (:0
          (Variables|Classes|SetArrowClass (Variables|Classes|GetPoisenArrowClass))
          (Variables|Money|SetSwitchAbility 1)
          (return (Variables|Money|GetPrice1.1ability)))
        (:1
          (Variables|Classes|SetArrowClass (Variables|Classes|GetFireArrowClass))
          (Variables|Money|SetSwitchAbility 2)
          (return (Variables|Money|GetPrice1.2ability)))))))

(fn HasEnoughMoney
  (bind _asgameplay_pc (Utilities|Casting|CastToGameplayPC (Game|GetInstigatorController)))
  (Variables|Default|SetPlayerController _asgameplay_pc)
  (Variables|Money|SetMoney (.Money (Utilities|Struct|BreakPlayerKD (Variables|/Game/Blueprints/Gameplay/GameplayPC.GameplayPC_C|GetPlayerKD _asgameplay_pc))))
  (switch int (Variables|Money|GetSwitchAbility)
    (:0
      (if (>= (Variables|Money|GetMoney) (Variables|Money|GetPrice1.1ability))
        _
        (else
          (Development|PrintString "No enough money" true true "(R=0.951458,G=1.000000,B=0.000000,A=1.000000)" 5.0 :!label _label)
          (return false))))
    (:1
      (if (>= (Variables|Money|GetMoney) (Variables|Money|GetPrice1.2ability))
        _
        (else
          (goto _label)))))
  (return true))